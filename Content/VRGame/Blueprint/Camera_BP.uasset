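; Grabbable VR camera that takes photos and turns them into picture actors.
; While not held, it snaps to the VRCharacter's CameraPosition on BeginPlay, on drop and every Tick.
; ScreenCamera captures the TakePhoto component into a fresh render target and returns it wrapped in a dynamic material instance.
; CreatePicture spawns a Picture_BP at the character's PictureSpawn and applies a given material to its Photo, with neither function called in this file.
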(event `self.ReceiveBeginPlay`
  (bind _returnvalue (`GameplayStatics.GetActorOfClass` "/Game/VRTemplate/Blueprints/VRCharacter.VRCharacter_C" :!label _label))
  (`/Engine/EditorBlueprintResources/StandardMacros.IsValid` _returnvalue
    (:`Is Valid`
      (bind _cameraposition (`/Game/VRTemplate/Blueprints/VRCharacter.CameraPosition` _returnvalue))
      (`self.K2_SetActorLocation` (`SceneComponent.K2_GetComponentLocation` _cameraposition))
      (`self.K2_SetActorRotation` (`SceneComponent.K2_GetComponentRotation` _cameraposition) true))))

(event `self.GrabComponent.OnDropped`
  (goto _label))

(event `self.ReceiveTick`
  (params (DeltaSeconds :type "Float (single-precision)"))
  (if (not (`/Game/VRTemplate/Blueprints/GrabComponent.bIsHeld` (`self.GrabComponent`)))
    (goto _label)))

(fn `CreatePicture`
  (params (Material :type "MaterialInstanceDynamic Object Reference"))
  (bind _returnvalue (`GameplayStatics.GetActorOfClass` "/Game/VRTemplate/Blueprints/VRCharacter.VRCharacter_C"))
  (bind _picturespawn (`/Game/VRTemplate/Blueprints/VRCharacter.PictureSpawn` _returnvalue))
  (bind _returnvalue_2 (`|SpawnActorFromClass` "/Game/VRGame/Blueprint/Picture_BP.Picture_BP_C" (`KismetMathLibrary.MakeTransform` (`SceneComponent.K2_GetComponentLocation` _picturespawn) (`SceneComponent.K2_GetComponentRotation` _picturespawn)) "Undefined" "MultiplyWithRoot" null null))
  (`PrimitiveComponent.SetMaterial` (`/Game/VRGame/Blueprint/Picture_BP.Photo` _returnvalue_2) 0 Material))

(fn `ScreenCamera`
  (returns (Material :type "MaterialInstanceDynamic Object Reference"))
  (bind _take_photo (`self.Take Photo`))
  (bind _returnvalue (`KismetRenderingLibrary.CreateRenderTarget2D` 512 512))
  (bind _returnvalue_2 (`KismetMaterialLibrary.CreateDynamicMaterialInstance` "/Game/VRGame/Materials/PhotoCamera_MatInstance.PhotoCamera_MatInstance"))
  (`MaterialInstanceDynamic.SetTextureParameterValue` _returnvalue_2 "Param" _returnvalue)
  (set `SceneCaptureComponent2D.TextureTarget` _returnvalue _take_photo)
  (`SceneCaptureComponent2D.CaptureScene` _take_photo)
  (return _returnvalue_2))

(fn `UserConstructionScript`)