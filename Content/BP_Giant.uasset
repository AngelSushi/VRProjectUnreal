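; BP_Giant is a giant whose gaze sweeps along the level's BP_Spline from BeginPlay and reacts to the VR player.
; A timeline moves WayPoint along the spline, turns Sight toward that point and sphere-traces from SightRoot to it, using local-space spline transforms as world values.
; When the trace hits BP_VRCharacter and its PlayerTrace returns false, it calls SpawnWall facing the player.
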(event `self.ReceiveBeginPlay`
  (bind _returnvalue (`GameplayStatics.GetActorOfClass` "/Game/BP_Spline.BP_Spline_C"))
  (set `self.BP_Spline` _returnvalue)
  (`self.StartMoving`))

(event `StartMoving`
  (bind _returnvalue (`SceneComponent.K2_GetComponentLocation` (`self.SightRoot`)))
  (bind (_direction _alphavalue) (`Timeline|SplineTimeline`)
    (:`Update`
      (bind _returnvalue_2 (`SplineComponent.GetTransformAtDistanceAlongSpline` (`/Game/BP_Spline.Spline` (`self.BP_Spline`)) (`KismetMathLibrary.Lerp` 0.0 (`SplineComponent.GetSplineLength` (`/Game/BP_Spline.Spline` (`self.BP_Spline`))) _alphavalue) "Local" false))
      (`SceneComponent.K2_SetWorldTransform` (`self.WayPoint`) _returnvalue_2 false false)
      (bind _location (.location _returnvalue_2))
      (`SceneComponent.K2_SetWorldRotation` (`self.Sight`) (`KismetMathLibrary.FindLookAtRotation` _returnvalue _location) false false)
      (bind _outhit (`KismetSystemLibrary.SphereTraceSingle` _returnvalue _location 250.0 "TraceTypeQuery5"))
      (bind _asbp_vrcharacter (cast `/Game/VRTemplate/Blueprints/BP_VRCharacter` (`.HitActor` (`GameplayStatics.BreakHitResult` _outhit))))
      (bind _monsterhit (`/Game/VRTemplate/Blueprints/BP_VRCharacter.PlayerTrace` _asbp_vrcharacter))
      (`KismetSystemLibrary.PrintString` "Oh playerTrace haha")
      (if (not _monsterhit)
        (bind _returnvalue_3 (`self.K2_GetActorLocation` _asbp_vrcharacter))
        (bind _returnvalue_4 (* (- _returnvalue_3 (`self.GetActorForwardVector` _asbp_vrcharacter)) (`self.Distance`)))
        (`self.SpawnWall` _returnvalue_4 (`KismetMathLibrary.FindLookAtRotation` _returnvalue_4 _returnvalue_3))))))

(fn `UserConstructionScript`)